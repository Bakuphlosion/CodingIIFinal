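; BP_SecCamera is a security camera that detects targets through AI Perception and reports to the shared BP_SecurityInstance game instance.
; Each perception update writes the stimulus location there as the player location.
; A successful sense is rechecked after a short delay before setting the detection flag, while losing sight clears it.
; Debug prints and a red box at the stimulus location show both outcomes.
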(event `self.AIPerception.OnTargetPerceptionUpdated`
  (params (Actor :type "Actor Object Reference") (Stimulus :type "AIStimulus Structure"))
  (bind (_age _expirationage _strength _stimuluslocation _receiverlocation _tag _bsuccessfullysensed) (break `AIStimulus` Stimulus))
  (bind _asbp_security_instance (cast `/Game/BP_SecurityInstance` (`GameplayStatics.GetGameInstance`)))
  (set `/Game/BP_SecurityInstance.PlayerLocation` _stimuluslocation _asbp_security_instance)
  (if _bsuccessfullysensed
    (`KismetSystemLibrary.PrintString` "I see something" true true (struct :`R` 1.0 :`G` 0.899544 :`A` 1.0))
    (`KismetSystemLibrary.Delay` 2.0)
    (if _bsuccessfullysensed
      (`KismetSystemLibrary.PrintString` "Calling Guards")
      (set `/Game/BP_SecurityInstance.DetectsPlayer` true _asbp_security_instance)
      (`KismetSystemLibrary.DrawDebugBox` _stimuluslocation (0.0 0.0 0.0) (struct :`R` 1.0 :`B` 0.069188 :`A` 1.0) (struct) 30.0 50.0 :!label _label))
    (else
      (`KismetSystemLibrary.PrintString` "I no longer see the thing" true true (struct :`R` 1.0 :`B` 0.021375 :`A` 1.0))
      (set `/Game/BP_SecurityInstance.DetectsPlayer` false _asbp_security_instance)
      (goto _label))))

(fn `UserConstructionScript`)