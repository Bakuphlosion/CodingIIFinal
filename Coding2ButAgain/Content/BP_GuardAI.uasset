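; Guard AI that investigates locations, patrols, chases seen pawns and catches the player at close range.
; Investigate moves to a given destination, then steps through supplied patrol points before returning to the start position.
; PawnSensing triggers a chase to the pawn's location at that moment, then a delayed return to station.
; A looping BeginPlay distance check calls Caught on the player character, while overhead text shows the current state.
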(event `self.ReceiveBeginPlay`
  (if true
    (`TextRenderComponent.K2_SetText` (`self.TextRender`) (`KismetTextLibrary.Conv_StringToText` "Waiting")))
  (set `self.StartLocation` (`SceneComponent.K2_GetComponentLocation` (`self.CapsuleComponent`)))
  (if (<= (`KismetMathLibrary.Vector_Distance` (`SceneComponent.K2_GetComponentLocation` (`self.CapsuleComponent`)) (`SceneComponent.K2_GetComponentLocation` (`Character.CapsuleComponent` (`GameplayStatics.GetPlayerCharacter` 0)))) 100.0) :!label _label
    (`KismetSystemLibrary.PrintString` "Gotcha!")
    (bind _asbp_first_person_character (cast `/Game/FirstPerson/Blueprints/BP_FirstPersonCharacter` (`GameplayStatics.GetPlayerCharacter` 0)))
    (`/Game/FirstPerson/Blueprints/BP_FirstPersonCharacter.Caught` _asbp_first_person_character)
    (`KismetSystemLibrary.Delay` 3.0)
    (goto _label)
    (else
      (`KismetSystemLibrary.Delay` 0.2)
      (goto _label))))

(event `Investigate`
  (params (Destination :type "Vector Structure") (PatrolPoints :type "Array of Actor Object Reference"))
  ;[1 1 1] Investigate
  (if (`self.Debugging`)
    (`TextRenderComponent.K2_SetText` (`self.TextRender`) (`KismetTextLibrary.Conv_StringToText` "Investigate")))
  (set `self.PatrolPoints` PatrolPoints)
  (set `self.Index` 0)
  (`KismetSystemLibrary.PrintString` (`KismetStringLibrary.Concat_StrStr` "Im going to " (`KismetStringLibrary.Conv_VectorToString` Destination)) true true (struct :`G` 0.66 :`B` 1.0 :`A` 1.0) 10.0)
  (`|AIMoveTo` self Destination null 50.0
    (:`OnSuccess`
      (`KismetSystemLibrary.Delay` 2.0)
      (if (not (`self.Chasing`))
        (`self.Patrol`)))))

(event `Patrol`
  ;[1 1 1] Go on patrol
  (if (`self.Debugging`)
    (`TextRenderComponent.K2_SetText` (`self.TextRender`) (`KismetTextLibrary.Conv_StringToText` "Patrol")))
  (`|AIMoveTo` self (0.0 0.0 0.0) (`|GetArrayItem` (`self.PatrolPoints`) (`self.Index`)) 100.0 :!label _label_2
    (:`OnSuccess`
      _)
    (:`OnFail`
      _))
  (`KismetSystemLibrary.Delay` 2.0)
  (`/Engine/EditorBlueprintResources/StandardMacros.IncrementInt` (`self.Index`)
    (:`  `
      (if (`self.Chasing`)
        _
        (elif (>= (`self.Index`) (`KismetArrayLibrary.Array_Length` (`self.PatrolPoints`)))
          (`self.ReturnToStation`)
          (else
            (goto _label_2)))))))

(event `ReturnToStation`
  ;[1 1 1] Go back to my station
  (if true
    (`TextRenderComponent.K2_SetText` (`self.TextRender`) (`KismetTextLibrary.Conv_StringToText` "Return")))
  (`|AIMoveTo` self (`self.StartLocation`) null 100.0))

(event `Chase`
  ;[1 1 1] Chase when I see the player
  (if (`self.Debugging`)
    (`TextRenderComponent.K2_SetText` (`self.TextRender`) (`KismetTextLibrary.Conv_StringToText` "Chase")))
  (set `self.Chasing` true)
  (`|AIMoveTo` self (`self.K2_GetActorLocation` (stale `self.PawnSensing.OnSeePawn` Pawn)) null 10.0
    (:`OnSuccess`
      _)
    (:`OnFail`
      _))
  (switch `EPathFollowingResult` "Success"
    (:`Success`
      (`KismetSystemLibrary.PrintString` "moveto success"))
    (:`Blocked`
      _)
    (:`OffPath`
      _)
    (:`Invalid`
      _))
  (`KismetSystemLibrary.Delay` 3.0)
  (set `self.Chasing` false)
  (`self.ReturnToStation`))

(event `self.PawnSensing.OnSeePawn`
  (params (Pawn :type "Pawn Object Reference"))
  ;[1 1 1] Chase when I see the player
  (`self.Chase`))

(fn `UserConstructionScript`)