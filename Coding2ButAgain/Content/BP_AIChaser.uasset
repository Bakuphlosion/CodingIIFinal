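; BP_AIChaser is an AI pawn that chases the player once a shared security state reports the player as detected.
; Each Tick it reads the detection flag and player location from BP_SecurityInstance, the game instance, and issues AI MoveTo toward that location.
; When the player is not detected, it waits on a Delay, then moves back to the capsule location saved at BeginPlay.
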(event `self.ReceiveBeginPlay`
  (set `self.StartLocation` (`SceneComponent.K2_GetComponentLocation` (`self.CapsuleComponent`))))

(event `self.ReceiveTick`
  (params (DeltaSeconds :type "Float (single-precision)"))
  (bind _asbp_security_instance (cast `/Game/BP_SecurityInstance` (`GameplayStatics.GetGameInstance`)))
  (if (`/Game/BP_SecurityInstance.DetectsPlayer` _asbp_security_instance)
    (`|AIMoveTo` self (`/Game/BP_SecurityInstance.PlayerLocation` _asbp_security_instance) null)
    (else
      (`KismetSystemLibrary.Delay` 3.0)
      (`|AIMoveTo` self (`self.StartLocation`) null))))

(fn `UserConstructionScript`)