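; BP_SecCam2 is a security camera that spots the player through AI Perception and alerts guards.
; When a BP_FirstPersonCharacter is sensed, it waits one second, rechecks the stimulus, then calls Investigate on every BP_GuardAI sharing its GroupID.
; Each guard receives the player's location and the camera's PatrolPoints.
; Debug prints and boxes mark where the player is reported or lost.
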(event `self.AIPerception.OnTargetPerceptionUpdated`
  (params (Actor :type "Actor Object Reference") (Stimulus :type "AIStimulus Structure"))
  (bind (_age _expirationage _strength _stimuluslocation _receiverlocation _tag _bsuccessfullysensed) (break `AIStimulus` Stimulus))
  (bind _asbp_first_person_character (cast `/Game/FirstPerson/Blueprints/BP_FirstPersonCharacter` Actor)) ; Are we seeing the player?
  (if _bsuccessfullysensed
    (bind _returnvalue (`SceneComponent.K2_GetComponentLocation` (`Character.CapsuleComponent` _asbp_first_person_character)))
    (`KismetSystemLibrary.PrintString` (`KismetStringLibrary.Concat_StrStr` "I see something at " (`KismetStringLibrary.Conv_VectorToString` _returnvalue)) true true (struct :`R` 1.0 :`G` 0.899544 :`A` 1.0) 10.0)
    (`KismetSystemLibrary.Delay` 1.0)
    (if _bsuccessfullysensed
      (`KismetSystemLibrary.PrintString` "Calling Guards")
      (`KismetSystemLibrary.DrawDebugBox` _returnvalue (0.0 0.0 0.0) (struct :`G` 1.0 :`B` 0.349876 :`A` 1.0) (struct) 30.0 50.0)
      (bind _outactors (`GameplayStatics.GetAllActorsOfClass` "/Game/BP_GuardAI.BP_GuardAI_C"))
      (for _array_element _outactors
        (if (== (`self.GroupID`) (`/Game/BP_GuardAI.GroupID` _array_element))
          (`/Game/BP_GuardAI.Investigate` _array_element _returnvalue (`self.PatrolPoints`)))))
    (else
      (`KismetSystemLibrary.PrintString` "I no longer see the thing" true true (struct :`R` 1.0 :`B` 0.021375 :`A` 1.0))
      (`KismetSystemLibrary.DrawDebugBox` _returnvalue (0.0 0.0 0.0) (struct :`R` 1.0 :`B` 0.069188 :`A` 1.0) (struct) 30.0 50.0))))

(fn `UserConstructionScript`)